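; BP_PlayerState holds the player's HP and a Box counter for the hack-and-slash game.
; AddDamge subtracts damage while CurHp is above zero, without broadcasting the change.
; Only a call made when HP is already at or below zero fires the UpdateHp and Death dispatchers, so the killing hit itself announces nothing.
; AddBox increments the Box count by one.
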(event EventBeginPlay)

(event EventTick
  (params (DeltaSeconds :type Float%20%28single-precision%29)))

(fn ConstructionScript)

(fn AddDamge
  (params (Damage :type Float%20%28double-precision%29))
  (if (CallFunction|IsDeath)
    (Default|CallEventDispatcherUpdateHp (stale _output_get) (Variables|Default|GetMaxHp))
    (if (<= (Variables|Default|GetCurHp) 0.0)
      (Default|CallEventDispatcherDeath))
    (else
      (bind _output_get (Variables|Default|SetCurHp (- (Variables|Default|GetCurHp) Damage))))))

(fn IsDeath
  (return (<= (Variables|Default|GetCurHp) 0.0)))

(fn AddBox
  (Variables|Default|SetBox (+ (Variables|Default|GetBox) 1)))