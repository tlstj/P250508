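; BP_BoxBase is a box item that can credit a BP_Wizard's player state via AddBox and then destroy itself.
; Its mesh's overlap events set a flag for any actor, and Tick accumulates time while it is set, resetting otherwise.
; The over-three-second threshold is checked only when an overlap begins, not in Tick, so staying inside alone does not trigger collection.
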(event OnComponentBeginOverlap(StaticMesh)
  (params (OverlappedComponent :type Primitive%20Component%20Object%20Reference) (OtherActor :type Actor%20Object%20Reference) (OtherComp :type Primitive%20Component%20Object%20Reference) (OtherBodyIndex :type Integer) (bFromSweep :type Boolean) (SweepResult :type Hit%20Result%20Structure%20%28by%20ref%29))
  (Variables|Default|SetIsOverlap true)
  (bind _asbp_wizard (Utilities|Casting|CastToBP_Wizard OtherActor))
  (bind _asbp_player_state (Utilities|Casting|CastToBP_PlayerState (Variables|/Script/Engine.Pawn|GetPlayerState _asbp_wizard)))
  (if (> (Variables|Default|GetTotalDeltaSecs) 3.0)
    (Default|AddBox _asbp_player_state)
    (Actor|DestroyActor)))

(event OnComponentEndOverlap(StaticMesh)
  (params (OverlappedComponent :type Primitive%20Component%20Object%20Reference) (OtherActor :type Actor%20Object%20Reference) (OtherComp :type Primitive%20Component%20Object%20Reference) (OtherBodyIndex :type Integer))
  (Variables|Default|SetIsOverlap false))

(event EventBeginPlay)

(event Collision|EventActorBeginOverlap
  (params (OtherActor :type Actor%20Object%20Reference)))

(event EventTick
  (params (DeltaSeconds :type Float%20%28single-precision%29))
  (if (Variables|Default|GetIsOverlap)
    (Variables|Default|SetTotalDeltaSecs (+ (* DeltaSeconds 1.0) (Variables|Default|GetTotalDeltaSecs)))
    (else
      (Variables|Default|SetTotalDeltaSecs 0.0))))

(fn ConstructionScript)