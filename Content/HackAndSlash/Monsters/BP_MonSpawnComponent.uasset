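; Monster spawner component that is meant to spawn an AI monster around its owning actor one second after BeginPlay.
; DoSpawn picks a point on a circle of 2π times Radius around the owner, then spawns the hard-coded "Cactus" class from DT_Monster with BT_Monster.
; IsCanSpawnLocation runs an upward line trace but always returns false, so no monster currently spawns.
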(event EventBeginPlay
  (Utilities|Time|SetTimerbyFunctionName 0 "DoSpawn" 1.0))

(event EventTick
  (params (DeltaSeconds :type Float%20%28single-precision%29)))

(fn DoSpawn
  (bind _output_get (LocalVariables|SetRandLocation (CallFunction|GetRandomCircleLoc)))
  (if (CallFunction|IsCanSpawnLocation _output_get)
    (DataTable|GetDataTableRowNames "/Game/HackAndSlash/Monsters/DT_Monster.DT_Monster")
    (bind _returnvalue (Utilities|GetDataTableRow "/Game/HackAndSlash/Monsters/DT_Monster.DT_Monster" "Cactus")
      (:then
        (AI|SpawnAIFromClass (.MonsterClass (Utilities|Struct|BreakST_Monster _returnvalue)) "/Game/HackAndSlash/AI/BT_Monster.BT_Monster" (LocalVariables|GetRandLocation) "0, 0, 0" false 0)))))

(fn GetRandomCircleLoc
  (bind _radius (Variables|Default|GetRadius))
  (bind _returnvalue (* _radius 2.0 3.141592))
  (bind _output_get (LocalVariables|SetRand (Math|Random|RandomFloatinRange 0.0 3.6e+02)))
  (return (+ (Transformation|GetActorLocation (Components|GetOwner)) (Math|Vector|MakeVector (* (Math|Trig|Cos(Radians) _output_get) _returnvalue) (* (Math|Trig|Sin(Radians) _output_get) _returnvalue) 0.0))))

(fn IsCanSpawnLocation
  (params (World%20Location :type Vector))
  (Collision|LineTraceForObjects World%20Location (+ World%20Location "0.000000,0.000000,100.000000") (Utilities|Array|MakeArray "ObjectTypeQuery1" "ObjectTypeQuery2") false 0 "None")
  (return false))